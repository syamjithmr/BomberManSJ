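; Blueprint game manager for a Bomberman-style game that cleans up bombs still in the level when a match is won or drawn.
; GameWon and GameDraw call their parent logic, then refund each live Bomb to its owning player's AvailableBombs and clear the Bomb_BP blast timer.
; Both paths then converge on UpdatePlayerStats, called on the BomberManSJGameManager actor found in the level.
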(event `self.GameDraw`
  ;[1 1 1] Resets the timer and disables any Bomb present in the level after Win/Draw.
  (`parent.GameDraw`)
  (bind _outactors (`GameplayStatics.GetAllActorsOfClass` "/Script/BomberManSJ.Bomb"))
  (for _array_element _outactors
    (`/Engine/EditorBlueprintResources/StandardMacros.IncrementInt` (`BomberManSJCharacter.AvailableBombs` (`Bomb.ParentPlayer` _array_element))
      (:`  `
        (bind _asbomb_bp (cast `/Game/Blueprints/Bomb_BP` _array_element))
        (`KismetSystemLibrary.K2_ClearAndInvalidateTimerHandle` (`/Game/Blueprints/Bomb_BP.BlastTimer` _asbomb_bp)))))
  (bind _returnvalue (`GameplayStatics.GetActorOfClass` "/Script/BomberManSJ.BomberManSJGameManager" :!label _label))
  (`self.UpdatePlayerStats` _returnvalue))

(event `self.GameWon`
  (params (Winner :type "BomberManSJCharacter Object Reference"))
  ;[1 1 1] Resets the timer and disables any Bomb present in the level after Win/Draw.
  (`parent.GameWon` Winner)
  (bind _outactors (`GameplayStatics.GetAllActorsOfClass` "/Script/BomberManSJ.Bomb"))
  (for _array_element _outactors
    (`/Engine/EditorBlueprintResources/StandardMacros.IncrementInt` (`BomberManSJCharacter.AvailableBombs` (`Bomb.ParentPlayer` _array_element))
      (:`  `
        (bind _asbomb_bp (cast `/Game/Blueprints/Bomb_BP` _array_element))
        (`KismetSystemLibrary.K2_ClearAndInvalidateTimerHandle` (`/Game/Blueprints/Bomb_BP.BlastTimer` _asbomb_bp)))))
  (goto _label))

(fn `UserConstructionScript`)