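; BombBlastEffect_BP is the bomb blast actor in a Bomberman-style game, handling whatever its collision box overlaps.
; It destroys breakable walls, ragdolls and kills characters, detonates other bombs immediately to chain blasts, and destroys other non-wall actors.
; When the particle system finishes, it destroys itself, activates any stored wall power-up, and has the game manager check player deaths if a kill occurred and no chain is flagged.
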(event `self.ReceiveBeginPlay`
  (bind _returnvalue (`GameplayStatics.GetActorOfClass` "/Script/BomberManSJ.BomberManSJGameManager"))
  (set `self.GameManager` _returnvalue))

(event `self.BoxCollission.OnComponentBeginOverlap`
  (params (OverlappedComponent :type "PrimitiveComponent Object Reference") (OtherActor :type "Actor Object Reference") (OtherComp :type "PrimitiveComponent Object Reference") (OtherBodyIndex :type Integer) (bFromSweep :type Boolean) (SweepResult :type "HitResult Structure (by ref)"))
  (bind _gamemanager (`self.GameManager`))
  (bind _aswall_base (cast `WallBase` OtherActor)
    (:`then`
      (if (`WallBase.IsBreakabale` _aswall_base)
        (set `self.PowerUp` (`WallBase.PowerUp` _aswall_base))
        (`self.K2_DestroyActor` _aswall_base)))
    (:`CastFailed`
      (bind _asbomber_man_sjcharacter (cast `BomberManSJCharacter` OtherActor)
        (:`then`
          (set `BomberManSJCharacter.IsDead` true _asbomber_man_sjcharacter)
          (bind _mesh (`Character.Mesh` _asbomber_man_sjcharacter))
          (`PrimitiveComponent.SetCollisionProfileName` _mesh "Ragdoll" true)
          (`PrimitiveComponent.SetSimulatePhysics` _mesh true)
          (set `BomberManSJGameManager.BlastKilledOne` true _gamemanager))
        (:`CastFailed`
          (bind _asbomb (cast `Bomb` OtherActor)
            (:`then`
              (bind _asbomb_bp (cast `/Game/Blueprints/Bomb_BP` _asbomb))
              (`KismetSystemLibrary.K2_ClearAndInvalidateTimerHandle` (`/Game/Blueprints/Bomb_BP.BlastTimer` _asbomb_bp))
              (set `/Game/Blueprints/Bomb_BP.TimeTillExplosion` 0 _asbomb_bp)
              (set `BomberManSJGameManager.BlastIsChained` true _gamemanager)
              (`/Game/Blueprints/Bomb_BP.Blast` _asbomb_bp))
            (:`CastFailed`
              (set `BomberManSJGameManager.BlastIsChained` false _gamemanager)
              (`self.K2_DestroyActor` OtherActor))))))))

(event `self.P_BombBlast.OnSystemFinished`
  (params (PSystem :type "ParticleSystemComponent Object Reference"))
  (bind _gamemanager (`self.GameManager`))
  (bind _powerup (`self.PowerUp`))
  (`self.K2_DestroyActor`)
  (if (`KismetSystemLibrary.IsValid` _powerup)
    (`PowerUpBase.ActivatePowerUp` _powerup))
  (if (and (not (`BomberManSJGameManager.BlastIsChained` _gamemanager)) (`BomberManSJGameManager.BlastKilledOne` _gamemanager))
    (set `BomberManSJGameManager.BlastKilledOne` false _gamemanager)
    (set `BomberManSJGameManager.BlastIsChained` false _gamemanager)
    (`BomberManSJGameManager.CheckPlayersDeadStatus` _gamemanager)))

(fn `UserConstructionScript`)