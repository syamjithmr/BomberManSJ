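; Bomb actor that detonates on a three-second timer started at BeginPlay.
; Blast turns off overlap events on the bomb mesh and spawns a blast effect actor at each entry in BlastLocations.
; It then returns one available bomb to the ParentPlayer's count and destroys itself.
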(event `self.ReceiveBeginPlay`
  (bind _returnvalue (`KismetSystemLibrary.K2_SetTimer` null "Blast" 3.0))
  (set `self.BlastTimer` _returnvalue))

(fn `Blast`
  (bind _parentplayer (`self.ParentPlayer`))
  (set `PrimitiveComponent.bGenerateOverlapEvents` false (`self.BombMesh`))
  (for _array_element (`self.BlastLocations`)
    (`|SpawnActorFromClass` "/Game/Blueprints/BombBlastEffect_BP.BombBlastEffect_BP_C" (`KismetMathLibrary.Conv_VectorToTransform` _array_element) "Undefined" "OverrideRootScale" null null))
  (set `BomberManSJCharacter.AvailableBombs` (+ (`BomberManSJCharacter.AvailableBombs` _parentplayer) 1) _parentplayer)
  (`self.K2_DestroyActor`))

(fn `UserConstructionScript`)